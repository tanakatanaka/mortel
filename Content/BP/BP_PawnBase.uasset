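; BP_PawnBase is a pawn Blueprint that provides a helper for reading the mouse cursor's angle around its Sphere component.
; FnGetDegrees deprojects the cursor into a long world ray and line-traces it against the Sphere alone.
; On a hit, it converts the point to the Sphere's local space and returns the XY atan2 angle in degrees with a hit flag.
; The event graph and construction script are empty.
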(event `Key|LeftMouseButton`
  (params (Key :type "Key Structure")))

(fn `Fn Get Degrees`
  (returns (isHit :type Boolean) (degrees :type "Float (double-precision)"))
  (bind _returnvalue (`GameplayStatics.GetPlayerController` 0))
  (bind (_locationx _locationy) (`PlayerController.GetMousePosition` _returnvalue))
  (bind (_worldposition _worlddirection) (`GameplayStatics.DeprojectScreenToWorld` _returnvalue (`KismetMathLibrary.MakeVector2D` _locationx _locationy)))
  (bind (_hitlocation _hitnormal _bonename _outhit _returnvalue_2) (`PrimitiveComponent.K2_LineTraceComponent` (`self.Sphere`) _worldposition (+ _worldposition (* _worlddirection 10000)) true false false))
  (if _returnvalue_2
    (bind (_returnvalue_x _returnvalue_y) (`KismetMathLibrary.BreakVector` (`KismetMathLibrary.InverseTransformLocation` (`SceneComponent.K2_GetComponentToWorld` (`self.Sphere`)) _hitlocation)))
    (return true (`KismetMathLibrary.DegAtan2` _returnvalue_y _returnvalue_x))
    (else
      (return false 0.0))))

(fn `UserConstructionScript`)